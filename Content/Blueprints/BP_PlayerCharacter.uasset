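; BP_PlayerCharacter is the player character Blueprint, which triggers a sprint through the Gameplay Ability System.
; Pressing Q checks that the Ability System Component is valid, then tries to activate GA_Sprint by class with remote activation allowed.
; BeginPlay, Tick and the construction script are empty.
; Unconnected debug nodes would print the RPGPlayerState's ability component active state and stamina, but never run.
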(event EventBeginPlay)

(event Collision|EventActorBeginOverlap
  (params (OtherActor :type Actor%20Object%20Reference)))

(event EventTick
  (params (DeltaSeconds :type Float%20%28single-precision%29)))

(event Input|KeyboardEvents|Q
  (params (Key :type Key%20Structure))
  (bind _returnvalue (Class|RPGCharacter|GetAbilitySystemComponent))
  (:Pressed
    (Utilities|IsValid _returnvalue
      (:Is%20Valid
        (Abilities|TryActivateAbilitybyClass _returnvalue "/Game/Abilities/Sprint/GA_Sprint.GA_Sprint_C" true)))))

(fn ConstructionScript)